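; Player controller that handles the pause menu and inventory screen, each toggled by an input action and pausing the game.
; Pause alternates through a FlipFlop and is ignored while the inventory is open; inventory tracks an open flag and does not check for an active pause menu.
; Both widgets are created on first use, cached, then added to or removed from the viewport.
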(event Input|ActionEvents|InputActionPauseGame
  (params (Key :type Key%20Structure))
  ;[1 1 1] Pause Game
  (:Pressed
    (if (not (Variables|Default|GetibInventoryOpen))
      (Utilities|FlowControl|FlipFlop
        (:A
          (bind _returnvalue (Game|SetGamePaused true))
          (if _returnvalue
            (Utilities|IsValid (Variables|Default|GetPauseWidget)
              (:Is%20Valid
                _)
              (:Is%20Not%20Valid
                (bind _returnvalue_2 (UserInterface|CreateWidget "/Game/UI/WB_Pause.WB_Pause_C"))
                (bind _output_get (Variables|Default|SetPauseWidget _returnvalue_2))))
            (UserInterface|Viewport|AddtoViewport _output_get 0)
            (else
              (Development|PrintString "Failed to Pause Game"))))
        (:B
          (bind _returnvalue_3 (Game|SetGamePaused false))
          (if _returnvalue_3
            (Widget|RemovefromParent (Variables|Default|GetPauseWidget))
            (else
              (Development|PrintString "Failed to unpause Game"))))))))

(event Input|ActionEvents|InputActionOpenInventory
  (params (Key :type Key%20Structure))
  ;[1 1 1] Open Inventory
  (:Pressed
    (if (Variables|Default|GetibInventoryOpen)
      (Widget|RemovefromParent (Variables|Default|GetInventoryWidget))
      (Variables|Default|SetibInventoryOpen false)
      (Game|SetGamePaused false)
      (else
        (Utilities|IsValid (Variables|Default|GetInventoryWidget)
          (:Is%20Valid
            _)
          (:Is%20Not%20Valid
            (bind _returnvalue (UserInterface|CreateWidget "/Game/UI/Inventory/WB_Inventory.WB_Inventory_C"))
            (bind _output_get (Variables|Default|SetInventoryWidget _returnvalue))))
        (UserInterface|Viewport|AddtoViewport _output_get 0)
        (Variables|Default|SetibInventoryOpen true)
        (Game|SetGamePaused true)))))

(fn ConstructionScript)